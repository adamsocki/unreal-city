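; Player controller for a building-placement game that routes camera input to BP_CameraController and handles placing buildings with the mouse.
; Keys, axes and right-mouse drag drive camera movement, orbit, pitch and zoom.
; BeginPlay spawns a LogicManager, whose residential logic runs every Tick alongside a timer update and debug print.
; In placement mode, a cursor trace moves a preview actor, and left click spawns the building if valid; grid code is mostly disconnected.
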(event `self.ReceiveBeginPlay`
  (`self.InitManagers`))

(event `InputAxis|CameraOrbit`
  (params (AxisValue :type "Float (single-precision)"))
  (bind _asbp_camera_controller (cast `/Game/BP_CameraController` (`self.K2_GetPawn`)))
  (`/Game/BP_CameraController.CameraOrbit` _asbp_camera_controller AxisValue))

(event `InputAxis|MovementForward/Backward`
  (params (AxisValue :type "Float (single-precision)"))
  (bind _asbp_camera_controller (cast `/Game/BP_CameraController` (`self.K2_GetPawn`)))
  (`/Game/BP_CameraController.CameraForwardBackward` _asbp_camera_controller AxisValue))

(event `InputAxis|MovementLeft/Right`
  (params (AxisValue :type "Float (single-precision)"))
  (bind _asbp_camera_controller (cast `/Game/BP_CameraController` (`self.K2_GetPawn`)))
  (`/Game/BP_CameraController.CameraLeftRight` _asbp_camera_controller AxisValue))

(event `InputAction|CameraZoomIn`
  (params (Key :type "Key Structure"))
  (:`Pressed`
    (bind _asbp_camera_controller (cast `/Game/BP_CameraController` (`self.K2_GetPawn`)))
    (`/Game/BP_CameraController.CameraZoomIn` _asbp_camera_controller 1.0)))

(event `InputAction|CameraZoomOut`
  (params (Key :type "Key Structure"))
  (:`Pressed`
    (bind _asbp_camera_controller (cast `/Game/BP_CameraController` (`self.K2_GetPawn`)))
    (`/Game/BP_CameraController.CameraZoomOut` _asbp_camera_controller 1.0)))

(event `InputAxis|CameraPitch`
  (params (AxisValue :type "Float (single-precision)"))
  (bind _asbp_camera_controller (cast `/Game/BP_CameraController` (`self.K2_GetPawn`)))
  (`/Game/BP_CameraController.CameraPitch` _asbp_camera_controller AxisValue))

(event `InputAction|MouseRightClick`
  (params (Key :type "Key Structure"))
  (:`Pressed`
    (set `self.RightButtonPressed` true))
  (:`Released`
    (set `self.RightButtonPressed` false)))

(event `InputAxis|MouseX`
  (params (AxisValue :type "Float (single-precision)"))
  (if (`self.RightButtonPressed`)
    (bind _asbp_camera_controller (cast `/Game/BP_CameraController` (`self.K2_GetPawn`)))
    (`/Game/BP_CameraController.CameraOrbit` _asbp_camera_controller AxisValue)))

(event `InputAxis|MouseY`
  (params (AxisValue :type "Float (single-precision)"))
  (if (`self.RightButtonPressed`)
    (bind _asbp_camera_controller (cast `/Game/BP_CameraController` (`self.K2_GetPawn`)))
    (`/Game/BP_CameraController.CameraPitch` _asbp_camera_controller AxisValue)))

(event `self.ReceiveTick`
  (params (DeltaSeconds :type "Float (single-precision)"))
  (`self.UpdateDeltaTimer` DeltaSeconds)
  (bind _outactors (`GameplayStatics.GetAllActorsWithTag` "test"))
  (`KismetSystemLibrary.PrintString` (`KismetStringLibrary.Conv_IntToString` (`KismetArrayLibrary.Array_Length` _outactors)))
  (`/Game/LogicManager.residentialLogic` (`self.LogicManagerRef`))
  ;[1 1 1] PlacementFunction - BOOL
  (if (`self.PlacementModeEnabled`)
    (`self.UpdatePlacement`)))

(event `Key|LeftMouseButton`
  (params (Key :type "Key Structure"))
  ;[1 1 1] PlacementFunction - BOOL
  (:`Pressed`
    (if (`self.PlacementModeEnabled`)
      (`self.SpawnBuilding`))))

(fn `InitManagers`
  (locals (ManagerTransform :type "Transform Structure"))
  (bind _output_get (set `local.ManagerTransform` (`KismetMathLibrary.MakeTransform` (0.0 0.0 -10000.0))))
  ;[1 1 1] Init - Logic Manager
  (bind _returnvalue (`|SpawnActorFromClass` "/Game/LogicManager.LogicManager_C" _output_get "Undefined" "OverrideRootScale" null null))
  (set `self.LogicManagerRef` _returnvalue))

(fn `MouseGridPosition`
  (params (GM :type "/Game/GridManager Object Reference"))
  (locals (NewLocalVar :type "Transform Structure"))
  (bind (_worldlocation _worlddirection) (`self.DeprojectMousePositionToWorld`))
  (bind _outhit (`KismetSystemLibrary.LineTraceSingle` _worldlocation (+ _worldlocation (* _worlddirection 10000.0)) "TraceTypeQuery3")))

(fn `SetPlacementModeEnabled`
  (params (IsEnabled :type Boolean))
  (bind _placeableactorref (`self.PlaceableActorRef`))
  (if (== IsEnabled (`self.PlacementModeEnabled`))
    (return)
    (else
      (bind _output_get (set `self.PlacementModeEnabled` IsEnabled))
      (if _output_get
        (bind _returnvalue (`|SpawnActorFromClass` (`/Game/MeshManagerComponent.placementActor` (`self.MeshManagerComponent`)) (`KismetMathLibrary.MakeTransform` (0.0 0.0 -10000.0)) "Undefined" "OverrideRootScale" null null))
        (bind _returnvalue_2 (`self.GetComponentByClass` _returnvalue "/Game/GameObjects/Components/MouseGrab.MouseGrab_C"))
        (`/Engine/EditorBlueprintResources/StandardMacros.IsValid` _returnvalue_2
          (:`Is Valid`
            (`/Game/GameObjects/Components/MouseGrab.InPlacementMode` _returnvalue_2))
          (:`Is Not Valid`
            _))
        (`AddComponent|NODE_AddPlaceableComponent-0`)
        (else
          ;[1 1 1] Destroy if Switched to False
          (`/Engine/EditorBlueprintResources/StandardMacros.IsValid` _placeableactorref
            (:`Is Valid`
              (`self.K2_DestroyActor` _placeableactorref))))))))

(fn `SpawnBuilding`
  (locals (NewLocalVar_0 :type "Actor Class Reference") (NewLocalVar_1 :type "Array of Name"))
  (bind _returnvalue (`self.GetComponentByClass` (`self.PlaceableActorRef`) "/Game/GameObjects/Components/PlaceableComponent.PlaceableComponent_C"))
  (bind _returnvalue_2 (`self.GetTransform` (`self.PlaceableActorRef`)))
  (`/Engine/EditorBlueprintResources/StandardMacros.IsValid` _returnvalue
    (:`Is Valid`
      (if (`/Game/GameObjects/Components/PlaceableComponent.IsPlacementValid` _returnvalue)
        (bind _returnvalue_3 (`|SpawnActorFromClass` (`self.ActorClassRef`) _returnvalue_2 "AlwaysSpawn" "OverrideRootScale" null null))
        (bind _returnvalue_4 (`AddComponent|NODE_AddBuildingComponent-0` :`self` _returnvalue_3))
        (set `ActorComponent.ComponentTags` (`local.NewLocalVar_1`) _returnvalue_4)
        (setmembers `/Game/GameObjects/Objects/BuildingData` :`StructRef` (`/Game/GameObjects/Components/BuildingComponent.BuildingData` _returnvalue_4) :`buildingType` "NewEnumerator0" :`transform` _returnvalue_2)
        (`self.SetPlacementModeEnabled` false)))))

(fn `UpdateDeltaTimer`
  (params (A :type "Float (double-precision)"))
  (set `self.myLogicData` (make `/Game/LogicData` 0 0 0 (+ A (`.residentialCreationTimer_10_CE15D798CE4612B7CB1783A72DE1E45F` (break `/Game/LogicData` (`self.myLogicData`)))))))

(fn `UpdatePlacement`
  (bind (_worldlocation _worlddirection) (`self.DeprojectMousePositionToWorld`))
  (bind _outhit (`KismetSystemLibrary.LineTraceSingle` _worldlocation (+ _worldlocation (* _worlddirection 10000.0)) "TraceTypeQuery3"))
  (bind (_bblockinghit _binitialoverlap _time _distance _location) (`GameplayStatics.BreakHitResult` _outhit))
  (if _bblockinghit
    (`self.K2_SetActorLocation` (`/Game/MeshManagerComponent.placementActorClass` (`self.MeshManagerComponent`)) _location false false)))

(fn `UserConstructionScript`)