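; Player-controllable camera pawn with a spring arm, supporting pan, orbit, pitch and zoom.
; BeginPlay moves the capsule to a fixed start position and applies the initial arm length.
; Input events pan along the spring arm's forward and right vectors and orbit through controller yaw.
; Pitch rotates the arm within clamped angles using the orbit speed, while zoom changes arm length without limits.
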(event `self.ReceiveBeginPlay`
  (`SceneComponent.K2_SetWorldLocation` (`self.CapsuleComponent`) (200.0 200.0 200.0) false false)
  (set `SpringArmComponent.TargetArmLength` (`self.ArmLength`) (`self.SpringArm`)))

(event `CameraLeftRight`
  (params (Movement :type "Float (double-precision)"))
  (`self.AddMovementInput` (`SceneComponent.GetRightVector` (`self.SpringArm`)) (* Movement (`self.MoveSpeed`))))

(event `CameraForwardBackward`
  (params (Magnitude :type "Float (double-precision)"))
  (`self.AddMovementInput` (`SceneComponent.GetForwardVector` (`self.SpringArm`)) (* Magnitude (`self.MoveSpeed`))))

(event `CameraOrbit`
  (params (Magnitude :type "Float (double-precision)"))
  (`self.AddControllerYawInput` (* Magnitude (`self.OrbitSpeed`))))

(event `CameraPitch`
  (params (Magnitude :type "Float (double-precision)"))
  (`SceneComponent.K2_SetWorldRotation` (`self.SpringArm`) (`KismetMathLibrary.Conv_VectorToRotator` (`KismetMathLibrary.Conv_RotatorToVector` (`KismetMathLibrary.MakeRotator` (.roll (`SceneComponent.K2_GetComponentRotation` (`self.SpringArm`))) (`KismetMathLibrary.ClampAngle` (+ (* (`self.OrbitSpeed`) Magnitude) (.pitch (`SceneComponent.K2_GetComponentRotation` (`self.SpringArm`)))) (`self.ClampAngleMin`) (`self.ClampAngleMax`)) (.yaw (`SceneComponent.K2_GetComponentRotation` (`self.SpringArm`)))))) false false))

(event `CameraZoomIn`
  (params (Magnitude :type "Float (double-precision)"))
  (bind _springarm (`self.SpringArm`))
  (set `SpringArmComponent.TargetArmLength` (- (`SpringArmComponent.TargetArmLength` _springarm) (* Magnitude (`self.ZoomSpeed`))) _springarm))

(event `CameraZoomOut`
  (params (Magnitude :type "Float (double-precision)"))
  (bind _springarm (`self.SpringArm`))
  (set `SpringArmComponent.TargetArmLength` (+ (`SpringArmComponent.TargetArmLength` _springarm) (* Magnitude (`self.ZoomSpeed`))) _springarm))

(fn `UserConstructionScript`)